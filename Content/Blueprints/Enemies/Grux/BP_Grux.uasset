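; BP_Grux is the Grux enemy Blueprint, which shows floating hit numbers when the ShowHitNumber event fires.
; That event creates a WBP_HitNumber widget with the damage, colored for headshots, projects it above the actor to screen space and plays its animation.
; Each widget and its world position go to StoreHitNumber, while UpdateHitNumberLocation reprojects a given position so the number can follow that world point on screen.
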(event `self.ShowHitNumber`
  (params (Damage :type Integer) (bIsHeadShot :type Boolean))
  (bind _returnvalue (+ (`self.K2_GetActorLocation`) (0.0 0.0 100.0)))
  (bind _returnvalue_2 (`|CreateWidget` "/Game/Blueprints/HUD/WBP_HitNumber.WBP_HitNumber_C"))
  (bind _hitnumbertext (`/Game/Blueprints/HUD/WBP_HitNumber.HitNumberText` _returnvalue_2))
  (`TextBlock.SetText` _hitnumbertext (`KismetTextLibrary.Conv_IntToText` Damage))
  (if bIsHeadShot
    (`TextBlock.SetColorAndOpacity` _hitnumbertext (make `SlateColor` (`self.HeadShotColor`))))
  (`CanvasPanelSlot.SetPosition` (`WidgetLayoutLibrary.SlotAsCanvasSlot` _hitnumbertext) (`WidgetLayoutLibrary.ProjectWorldLocationToWidgetPosition` (`GameplayStatics.GetPlayerController` 0) _returnvalue))
  (`UserWidget.AddToViewport` _returnvalue_2 0)
  (`UserWidget.PlayAnimationForward` _returnvalue_2 (`/Game/Blueprints/HUD/WBP_HitNumber.HitNumberAnimation` _returnvalue_2) 1.0 false)
  (`self.StoreHitNumber` _returnvalue_2 _returnvalue))

(event `self.UpdateHitNumberLocation`
  (params (HitNumber :type "UserWidget Object Reference") (Position :type "Vector Structure"))
  (bind _aswbp_hit_number (cast `/Game/Blueprints/HUD/WBP_HitNumber` HitNumber))
  (`CanvasPanelSlot.SetPosition` (`WidgetLayoutLibrary.SlotAsCanvasSlot` (`/Game/Blueprints/HUD/WBP_HitNumber.HitNumberText` _aswbp_hit_number)) (`WidgetLayoutLibrary.ProjectWorldLocationToWidgetPosition` (`GameplayStatics.GetPlayerController` 0) Position)))

(fn `UserConstructionScript`)